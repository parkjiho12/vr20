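; BP_moveLeftRight is an actor that moves its Plane component in a continuous square loop on the relative X and Z axes.
; Each Tick switches on the Selection state (Right, Up, Left, Down), steps the location one unit and advances the state at the 0 or 100 bound.
; Movement ignores delta time, so speed depends on frame rate.
; An unconnected Timeline that would slide the Plane along X never runs.
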(event EventBeginPlay)

(event Collision|EventActorBeginOverlap
  (params (OtherActor :type Actor%20Object%20Reference)))

(event EventTick
  (params (DeltaSeconds :type Float%20%28single-precision%29))
  (switch Utilities|FlowControl|Switch|SwitchonEN_MoveType (Variables|Default|GetSelection)
    (:NewEnumerator0
      (bind _output_get (Variables|Default|SetLocationX (+ (Variables|Default|GetLocationX) 1.0)))
      (Transformation|SetRelativeLocation (Variables|Default|GetPlane) (Math|Vector|MakeVector _output_get 0.0 (Variables|Default|GetLocationZ)) false false)
      (if (>= (Variables|Default|GetLocationX) 1e+02)
        (Variables|Default|SetSelection "NewEnumerator1")))
    (:NewEnumerator1
      (bind _output_get_2 (Variables|Default|SetLocationZ (+ (Variables|Default|GetLocationZ) 1.0)))
      (Transformation|SetRelativeLocation (Variables|Default|GetPlane) (Math|Vector|MakeVector (Variables|Default|GetLocationX) 0.0 _output_get_2) false false)
      (if (>= (Variables|Default|GetLocationZ) 1e+02)
        (Variables|Default|SetSelection "NewEnumerator2")))
    (:NewEnumerator2
      (bind _output_get_3 (Variables|Default|SetLocationX (- (Variables|Default|GetLocationX) 1.0)))
      (Transformation|SetRelativeLocation (Variables|Default|GetPlane) (Math|Vector|MakeVector _output_get_3 0.0 (Variables|Default|GetLocationZ)) false false)
      (if (<= (Variables|Default|GetLocationX) 0.0)
        (Variables|Default|SetSelection "NewEnumerator3")))
    (:NewEnumerator3
      (bind _output_get_4 (Variables|Default|SetLocationZ (- (Variables|Default|GetLocationZ) 1.0)))
      (Transformation|SetRelativeLocation (Variables|Default|GetPlane) (Math|Vector|MakeVector (Variables|Default|GetLocationX) 0.0 _output_get_4) false false)
      (if (<= (Variables|Default|GetLocationZ) 0.0)
        (Variables|Default|SetSelection "NewEnumerator0")))))

(fn ConstructionScript)